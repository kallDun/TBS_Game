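; BP_Grid_Grass_Test_Landscape_Gen is a grass grid cell for a landscape generation test map that adds its own landscape brush at runtime.
; On cell init it casts the LandscapeBrush child actor to a ShaderWorld brush and appends it as a new full-influence layer to the BP_BrushManager's runtime dynamic brush layers.
; The seed is fixed at zero, and the parent init call and grass-field PCG generation are left unconnected.
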(event EventOnCellInit
  (Utilities|FlowControl|Sequence
    (:then_0
      (bind _asshader_world_brush (Utilities|Casting|CastToShaderWorldBrush (Variables|/Script/Engine.ChildActorComponent|GetChildActor (Variables|Default|GetLandscape%20Brush)))))
    (:then_1
      (bind _returnvalue (Actor|GetActorOfClass "/ShaderWorld/BP/BP_BrushManager.BP_BrushManager_C"))
      (Utilities|Array|Add (Variables|/Script/ShaderWorld.ShaderWorldBrushManager|GetRuntimeDynamicBrushLayers _returnvalue) (Utilities|Struct|MakeBrushLayer true 1.0 (Utilities|Array|MakeArray (Utilities|Struct|MakeBrushElement true 1.0 _asshader_world_brush)))))))

(fn ConstructionScript)

(fn GenerateSeed
  (return 0))