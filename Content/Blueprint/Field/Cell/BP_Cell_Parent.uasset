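; Base Blueprint for field cells, providing a landscape brush and two world-space info widgets for building and general cell details.
; On BeginPlay, remote (non-authority) instances register their child-actor ShaderWorld brush as a runtime dynamic layer in BP_BrushManager, and both widgets are hidden.
; Show/hide events toggle each widget, initializing it with cell parameters or the cell and player.
; GeneratePCG is an empty event, with disconnected PCG setup nodes left in the graph.
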(event Custom|Show%20General%20Info
  (params (Player :type BP%20Player%20Controller%20Object%20Reference))
  (bind _widget_general_info (Variables|Default|GetWidget-General-Info))
  ;[0.3356 1 0.5439] General Info
  (Rendering|SetVisibility _widget_general_info true false)
  (bind _asw_cell_general_world_info (Utilities|Casting|CastToW_Cell_General_World_Info (UserInterface|GetWidget _widget_general_info)))
  (Default|Init _asw_cell_general_world_info self Player))

(event Custom|Hide%20General%20Info
  ;[0.3356 1 0.5439] General Info
  (Rendering|SetVisibility (Variables|Default|GetWidget-General-Info) false false))

(event Custom|Generate%20PCG
  (params (InGraph :type PCG%20Graph%20Interface%20Object%20Reference))
  ;[0.7552 1 0.2705] Init Procedural Generation
)

(event Custom|Init%20Landscape%20Brush
  ;[1 0.4422 0.0629] Init Landscape Brush
  (Networking|SwitchHasAuthority
    (:Remote
      (bind _asshader_world_brush (Utilities|Casting|CastToShaderWorldBrush (Variables|/Script/Engine.ChildActorComponent|GetChildActor (Variables|Default|GetLandscape%20Brush))))
      (bind _returnvalue (Actor|GetActorOfClass "/ShaderWorld/BP/BP_BrushManager.BP_BrushManager_C"))
      (Utilities|Array|Add (Variables|/Script/ShaderWorld.ShaderWorldBrushManager|GetRuntimeDynamicBrushLayers _returnvalue) (Utilities|Struct|MakeBrushLayer true 1.0 (Utilities|Array|MakeArray (Utilities|Struct|MakeBrushElement true 1.0 _asshader_world_brush)))))))

(event Custom|Show%20Building%20Info
  (params (Cell%20Params :type Cell%20Parameters%20Structure))
  (bind _widget_build_info (Variables|Default|GetWidget-Build-Info))
  ;[1 0.6788 0.1101] Build Info
  (Rendering|SetVisibility _widget_build_info true false)
  (bind _asw_cell_info (Utilities|Casting|CastToW_Cell_Info (UserInterface|GetWidget _widget_build_info)))
  (Default|Init _asw_cell_info Cell%20Params))

(event Custom|Hide%20Building%20Info
  ;[1 0.6788 0.1101] Build Info
  (Rendering|SetVisibility (Variables|Default|GetWidget-Build-Info) false false))

(event EventBeginPlay
  ;[1 0.5123 0.6747] Init
  (CallFunction|InitLandscapeBrush)
  (CallFunction|HideBuildingInfo)
  (CallFunction|HideGeneralInfo))

(fn ConstructionScript
  (|CallParentFunction))