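; Parent Blueprint for a building's view, which manages the info widget shown for that building.
; On init it takes the W_Building_Info from its Widget component and initializes it with itself and the BP_PlayerController from BuildingRef.
; Each tick it shows and updates that widget only while ViewState is Initialize, and hides it otherwise.
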(event Custom|Init%20Info%20Widget
  (bind _asw_building_info (Utilities|Casting|CastToW_Building_Info (UserInterface|GetWidget (Variables|Default|GetWidget))))
  (bind _output_get (Variables|Default|SetWidget%20Building%20Info _asw_building_info))
  (bind _asbp_player_controller (Utilities|Casting|CastToBP_PlayerController (Variables|/Script/TBS_Game.Building|GetPlayerControllerRef (Variables|Default|GetBuildingRef))))
  (Default|Init _output_get self _asbp_player_controller))

(event EventOnInit
  (CallFunction|InitInfoWidget))

(event EventTick
  (params (DeltaSeconds :type Float%20%28single-precision%29))
  (bind _viewstate (Variables|Default|GetViewState))
  (bind _widget_building_info (Variables|Default|GetWidget%20Building%20Info))
  (bind _returnvalue (Utilities|Enum|Equal(Enum) _viewstate "Initialize"))
  (Utilities|IsValid _widget_building_info
    (:Is%20Valid
      (Widget|SetVisibility _widget_building_info (select _returnvalue "Visible" "Hidden"))
      (if _returnvalue
        (Default|Update _widget_building_info)))))

(fn ConstructionScript)