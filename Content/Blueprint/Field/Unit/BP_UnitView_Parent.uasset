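; BP_UnitView_Parent is a parent Blueprint for a unit's view, holding a widget component for an info display.
; InitInfoWidget shows the W_Unit_Info widget and binds it to the view and player controller, but its only call here is unreachable.
; Tick calls UpdateWidgetState, which keeps a separately referenced building info widget hidden while updating it.
; OnInit and the BuildingRef rep-notify share an owner check that leads nowhere.
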(event Custom|Init%20Info%20Widget
  (bind _asw_unit_info (Utilities|Casting|CastToW_Unit_Info (UserInterface|GetWidget (Variables|Default|GetWidget))))
  (Rendering|SetVisibility (Variables|Default|GetWidget) true false)
  (bind _output_get (Variables|Default|SetWidget%20Unit%20Info _asw_unit_info))
  (bind _asbp_player_controller (Utilities|Casting|CastToBP_PlayerController (Variables|/Script/TBS_Game.Building|GetPlayerControllerRef (Variables|Default|GetUnitRef))))
  (Default|Init _output_get self _asbp_player_controller))

(event Custom|Update%20Widget%20State
  (bind _widget_building_info (Variables|Default|GetWidget%20Building%20Info))
  (Utilities|IsValid _widget_building_info
    (:Is%20Valid
      (Widget|SetVisibility _widget_building_info (select false "Visible" "Hidden"))
      (if true
        (Default|Update _widget_building_info)))))

(event Custom|OnRep_BuildingRef_1
  (Utilities|IsValid (Components|GetOwner)))

(event EventOnInit
  (Utilities|IsValid (Components|GetOwner)))

(event EventTick
  (params (DeltaSeconds :type Float%20%28single-precision%29))
  (Utilities|IsValid (Components|GetOwner)
    (:Is%20Valid
      (CallFunction|UpdateWidgetState))))

(fn ConstructionScript)