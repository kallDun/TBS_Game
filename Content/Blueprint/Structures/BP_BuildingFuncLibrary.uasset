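; Blueprint function library that packs a building's info, such as HP, cells, descriptions, requirements and properties, into one data structure for its current or a custom level.
; Above level 1, build moves, assemble moves and action info come from the upgrade component matching that level; otherwise they come from the building itself.
; GetComponentWithLevel finds that component, considering only ready components when the current level is used.
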(fn GetBuildingDataStructure
  (params (Building :type Building%20Object%20Reference) (Use%20Current%20Level :type Boolean) (Custom%20Level :type Integer))
  (bind _currentlevel (Variables|/Script/TBS_Game.Building|GetCurrentLevel Building))
  (bind _returnvalue (select Use%20Current%20Level _currentlevel Custom%20Level))
  (bind _upgrade_component (CallFunction|GetComponentwithLevel Building _returnvalue Use%20Current%20Level Building))
  (if (> _returnvalue 1)
    (return (Utilities|Struct|MakeS_BuildingData (Variables|/Script/TBS_Game.FieldActorsHandler|GetName Building) (Variables|/Script/TBS_Game.Building|GetBuildingType Building) (Variables|/Script/TBS_Game.Building|GetAffectingOnOtherBuildingImproveLevel Building) (Class|Building|GetMaxHitPoints Building Use%20Current%20Level Custom%20Level) (Utilities|Array|Length (Variables|/Script/TBS_Game.Building|GetBuildingViews Building)) (Class|Building|GetMaxCellCount Building Use%20Current%20Level Custom%20Level) (Variables|/Script/TBS_Game.UpgradeBuildingComponent|GetMovesToBuild _upgrade_component) (Variables|/Script/TBS_Game.UpgradeBuildingComponent|GetMovesToAssemble _upgrade_component) (Variables|/Script/TBS_Game.FieldActorsHandler|GetDescription Building) (Variables|/Script/TBS_Game.UpgradeBuildingComponent|GetUpgradeActionInfo _upgrade_component) (Variables|/Script/TBS_Game.Building|GetImproveLevelFromLocationInfo Building) (Variables|/Script/TBS_Game.Building|GetPropertyChangedFromImproveLevelInfo Building) (Variables|/Script/TBS_Game.FieldActorsHandler|GetLocationRequirementsInfo Building) (Variables|/Script/TBS_Game.FieldActorsHandler|GetMainRequirementsInfo Building) (Variables|/Script/TBS_Game.Building|GetRequirementsToExpendCells Building) (Class|Building|GetPropertiesbyLevel Building Use%20Current%20Level Custom%20Level)))
    (else
      (return (Utilities|Struct|MakeS_BuildingData (Variables|/Script/TBS_Game.FieldActorsHandler|GetName Building) (Variables|/Script/TBS_Game.Building|GetBuildingType Building) (Variables|/Script/TBS_Game.Building|GetAffectingOnOtherBuildingImproveLevel Building) (Class|Building|GetMaxHitPoints Building Use%20Current%20Level Custom%20Level) (Utilities|Array|Length (Variables|/Script/TBS_Game.Building|GetBuildingViews Building)) (Class|Building|GetMaxCellCount Building Use%20Current%20Level Custom%20Level) (Variables|/Script/TBS_Game.Building|GetMovesToBuild Building) (Variables|/Script/TBS_Game.Building|GetMovesToAssemble Building) (Variables|/Script/TBS_Game.FieldActorsHandler|GetDescription Building) (Variables|/Script/TBS_Game.Building|GetBuildActionInfo Building) (Variables|/Script/TBS_Game.Building|GetImproveLevelFromLocationInfo Building) (Variables|/Script/TBS_Game.Building|GetPropertyChangedFromImproveLevelInfo Building) (Variables|/Script/TBS_Game.FieldActorsHandler|GetLocationRequirementsInfo Building) (Variables|/Script/TBS_Game.FieldActorsHandler|GetMainRequirementsInfo Building) (Variables|/Script/TBS_Game.Building|GetRequirementsToExpendCells Building) (Class|Building|GetPropertiesbyLevel Building Use%20Current%20Level Custom%20Level))))))

(fn GetComponentwithLevel
  (params (Building :type Building%20Object%20Reference) (Level :type Integer) (OnlyReadyComponents :type Boolean))
  (for _array_element (Class|Building|GetUpgradeComponentswithLevel Building Level OnlyReadyComponents)
    (if (== (Variables|/Script/TBS_Game.UpgradeBuildingComponent|GetLevelNumber _array_element) Level)
      (return _array_element)))
  (return 0))