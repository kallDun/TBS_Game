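; BP_HUD_Controller creates the player's on-screen HUD and debug menu widgets and links the HUD to its player.
; On BeginPlay it adds both widgets to the viewport, casts the owning pawn to GamePlayerController, and subscribes to player-initialization-finished through the FieldController's TurnsOrderEventSystem.
; When that event reports this same player, it casts to BP_PlayerController and initializes the HUD and player with each other.
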(event Custom|PlayerInitializeFinished_Event
  (params (Player :type Game%20Player%20Controller%20Object%20Reference))
  (bind _hud (Variables|Default|GetHUD))
  (bind _as_game_player_controller (Variables|Default|GetAs%20Game%20Player%20Controller))
  (if (== Player _as_game_player_controller)
    (bind _asbp_player_controller (Utilities|Casting|CastToBP_PlayerController _as_game_player_controller))
    (Default|Init _hud _asbp_player_controller)
    (Default|InitHUD _asbp_player_controller _hud)))

(event EventBeginPlay
  (Utilities|FlowControl|Sequence
    (:then_0
      (bind _returnvalue (UserInterface|CreateWidget "/Game/Blueprint/Widget/UI/W_HUD.W_HUD_C"))
      (bind _output_get (Variables|Default|SetHUD _returnvalue))
      (UserInterface|Viewport|AddtoViewport _output_get 0))
    (:then_1
      (bind _returnvalue_2 (UserInterface|CreateWidget "/Game/Blueprint/Widget/DebugMenu/W_DebugMenu.W_DebugMenu_C"))
      (bind _output_get_2 (Variables|Default|SetDebugMenu _returnvalue_2))
      (UserInterface|Viewport|AddtoViewport _output_get_2 0))
    (:then_2
      (bind _asgame_player_controller (Utilities|Casting|CastToGamePlayerController (Class|HUD|GetOwningPawn)))
      (Variables|Default|SetAs%20Game%20Player%20Controller _asgame_player_controller)
      (EventDispatchers|AssignPlayerInitializeFinished (Variables|/Script/TBS_Game.FieldController|GetTurnsOrderEventSystem (Variables|/Script/TBS_Game.GamePlayerController|GetFieldController _asgame_player_controller)) (delegate Custom|PlayerInitializeFinished_Event)))))

(fn ConstructionScript)